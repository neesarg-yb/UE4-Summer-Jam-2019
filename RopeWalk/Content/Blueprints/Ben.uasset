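; Ben is a rope-walker actor that advances in steps along the level's single RopeSpline while swaying side to side.
; BeginPlay loads movement tuning from data tables and snaps Ben to the spline start.
; StepForward sets a new goal distance and speed multiplier, which Tick moves toward along the spline.
; Tick also oscillates a tilt angle while moving or always-swinging, shown only as a debug body line.
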(event `self.ReceiveBeginPlay`
  (bind _returnvalue_location (`KismetMathLibrary.BreakTransform` (`SplineComponent.GetTransformAtDistanceAlongSpline` (`/Game/Blueprints/RopeSpline.Spline` (`self.RopeSpline`)) 0.0 "World" false)))
  (`self.SetValuesFromDataTables`)
  (bind _outactors (`GameplayStatics.GetAllActorsOfClass` "/Game/Blueprints/RopeSpline.RopeSpline_C"))
  (for _array_element _outactors
    (set `self.RopeSpline` _array_element))
  (if (!= (`KismetArrayLibrary.Array_Length` _outactors) 1)
    (`KismetSystemLibrary.PrintString` "ERROR: Ben can work only with one Spline Rope! Just one!" true true (struct :`R` 1.0 :`B` 0.022518 :`A` 1.0) 10.0)
    (else
      (`KismetSystemLibrary.PrintString` "Ben has reference to the RopeSpline!" true true (struct :`G` 1.0 :`B` 0.207862 :`A` 1.0) 5.0)
      ;[1 1 1] Move to the start of the RopeSpline
      (`SceneComponent.K2_SetWorldLocation` (`self.DefaultSceneRoot`) _returnvalue_location false false))))

(event `self.ReceiveTick`
  (params (DeltaSeconds :type "Float (single-precision)"))
  (`self.UpdateCurrentDistance` DeltaSeconds)
  (`self.UpdateBenPosition`)
  (`self.UpdateBenSwing` DeltaSeconds)
  (`self.DebugRenderBodyLine`))

(fn `DebugRenderBodyLine`
  (locals (BodyLength :type "Float (double-precision)" :default 168.0))
  (bind _returnvalue (`SceneComponent.K2_GetComponentLocation` (`self.DefaultSceneRoot`)))
  (`KismetSystemLibrary.DrawDebugLine` _returnvalue (+ _returnvalue (`KismetMathLibrary.RotateAngleAxis` (`KismetMathLibrary.MakeVector` 0.0 0.0 (`local.BodyLength`)) (`self.CurrentVerticalOffsetDegrees`) (`SceneComponent.GetForwardVector` (`self.DefaultSceneRoot`)))) (struct :`G` 1.0 :`A` 1.0) 0.0 25.0))

(fn `SetValuesFromDataTables`
  (`|ExecutionSequence`
    (:`then_0`
      (bind _returnvalue (`|GetDataTableRow` "/Game/DataTables/BenMovement_Bools.BenMovement_Bools" "SwingConstantly")
        (:`then`
          (set `self.SwingConstantly` (break `/Game/DataStructures/BooleanStructure` _returnvalue)))
        (:`RowNotFound`
          (`KismetSystemLibrary.PrintString` "Warning: DATA TABLE ROW SwingConstantly NOT FOUND" true true (struct :`R` 1.0 :`B` 0.064835 :`A` 1.0) 5.0))))
    (:`then_1`
      (bind _returnvalue_2 (`|GetDataTableRow` "/Game/DataTables/BenMovement_Floats.BenMovement_Floats" "StepDistance")
        (:`then`
          (set `self.StepDistance` (break `/Game/DataStructures/FloatStructure` _returnvalue_2)))
        (:`RowNotFound`
          (`KismetSystemLibrary.PrintString` "Warning: DATA TABLE ROW StepDistance NOT FOUND" true true (struct :`R` 1.0 :`B` 0.064835 :`A` 1.0) 5.0))))
    (:`then_2`
      (bind _returnvalue_3 (`|GetDataTableRow` "/Game/DataTables/BenMovement_Floats.BenMovement_Floats" "WalkSpeedPerSecond")
        (:`then`
          (set `self.WalkSpeedPerSeconds` (break `/Game/DataStructures/FloatStructure` _returnvalue_3)))
        (:`RowNotFound`
          (`KismetSystemLibrary.PrintString` "Warning: DATA TABLE ROW WalkSpeedPerSec NOT FOUND" true true (struct :`R` 1.0 :`B` 0.064835 :`A` 1.0) 5.0))))
    (:`then_3`
      (bind _returnvalue_4 (`|GetDataTableRow` "/Game/DataTables/BenMovement_Floats.BenMovement_Floats" "LeftSwingMaxDegrees")
        (:`then`
          (set `self.LeftMaxSwingDegrees` (break `/Game/DataStructures/FloatStructure` _returnvalue_4)))
        (:`RowNotFound`
          (`KismetSystemLibrary.PrintString` "Warning: DATA TABLE ROW LeftMaxSwingDeg NOT FOUND" true true (struct :`R` 1.0 :`B` 0.064835 :`A` 1.0) 5.0))))
    (:`then_4`
      (bind _returnvalue_5 (`|GetDataTableRow` "/Game/DataTables/BenMovement_Floats.BenMovement_Floats" "RightSwingMaxDegrees")
        (:`then`
          (set `self.RightMaxSwingDegrees` (break `/Game/DataStructures/FloatStructure` _returnvalue_5)))
        (:`RowNotFound`
          (`KismetSystemLibrary.PrintString` "Warning: DATA TABLE ROW RightMaxSwingDeg NOT FOUND" true true (struct :`R` 1.0 :`B` 0.064835 :`A` 1.0) 5.0))))
    (:`then_5`
      (bind _returnvalue_6 (`|GetDataTableRow` "/Game/DataTables/BenMovement_Floats.BenMovement_Floats" "SwingSpeedPerSecond")
        (:`then`
          (set `self.SwingSpeedDegreesPerSeconds` (break `/Game/DataStructures/FloatStructure` _returnvalue_6)))
        (:`RowNotFound`
          (`KismetSystemLibrary.PrintString` "Warning: DATA TABLE ROW SwingSpeedPerSec NOT FOUND" true true (struct :`R` 1.0 :`B` 0.064835 :`A` 1.0) 5.0))))))

(fn `StepForward`
  (params (`Speed Multiplier` :type "Float (double-precision)"))
  (if (<= (`KismetMathLibrary.Square` (- (`self.CurrentDistanceOnRope`) (`self.GoalDistanceOnRope`))) 0.1)
    (set `self.CurrentSpeedMultiplier` `Speed Multiplier`)
    (set `self.GoalDistanceOnRope` (+ (`self.CurrentDistanceOnRope`) (`self.StepDistance`)))))

(fn `UpdateBenPosition`
  (bind (_returnvalue_location _returnvalue_rotation) (`KismetMathLibrary.BreakTransform` (`SplineComponent.GetTransformAtDistanceAlongSpline` (`/Game/Blueprints/RopeSpline.Spline` (`self.RopeSpline`)) (`self.CurrentDistanceOnRope`) "World" false)))
  (`SceneComponent.K2_SetWorldTransform` (`self.DefaultSceneRoot`) (`KismetMathLibrary.MakeTransform` _returnvalue_location _returnvalue_rotation) false false))

(fn `UpdateBenSwing`
  (params (DeltaSeconds :type "Float (double-precision)"))
  (locals (DeltaSwing :type "Float (double-precision)") (DeltaSec :type "Float (double-precision)"))
  (set `local.DeltaSec` DeltaSeconds)
  (if (or (`self.SwingConstantly`) (`self.IsBenMoving`))
    (`|ExecutionSequence`
      (:`then_0`
        ;[1 1 1] If reached Swing Direction MAX, flip the direction
        (switch `/Game/DataStructures/SwingDirection` (`self.SwingDirection`)
          (:`NewEnumerator0`
            (if (<= (`KismetMathLibrary.Square` (- (`self.CurrentVerticalOffsetDegrees`) (`self.LeftMaxSwingDegrees`))) 0.1)
              (set `self.SwingDirection` "NewEnumerator1")))
          (:`NewEnumerator1`
            (if (<= (`KismetMathLibrary.Square` (- (`self.CurrentVerticalOffsetDegrees`) (* (`self.RightMaxSwingDegrees`) -1.0))) 0.1)
              (set `self.SwingDirection` "NewEnumerator0")))))
      (:`then_1`
        ;[1 1 1] Calculate Delta Swing for this frame
        (switch `/Game/DataStructures/SwingDirection` (`self.SwingDirection`)
          (:`NewEnumerator0`
            (set `local.DeltaSwing` (* (`self.SwingSpeedDegreesPerSeconds`) (`local.DeltaSec`) 1.0)))
          (:`NewEnumerator1`
            (set `local.DeltaSwing` (* (`self.SwingSpeedDegreesPerSeconds`) (`local.DeltaSec`) -1.0)))))
      (:`then_2`
        (set `self.CurrentVerticalOffsetDegrees` (+ (`self.CurrentVerticalOffsetDegrees`) (`local.DeltaSwing`)))))))

(fn `UpdateCurrentDistance`
  (params (DeltaSeconds :type "Float (double-precision)"))
  (locals (DeltaSec :type "Float (double-precision)"))
  (set `local.DeltaSec` DeltaSeconds)
  (set `self.IsBenMoving` true)
  (if (< (`self.CurrentDistanceOnRope`) (`KismetMathLibrary.FClamp` (`self.GoalDistanceOnRope`) 0.0 (`SplineComponent.GetSplineLength` (`/Game/Blueprints/RopeSpline.Spline` (`self.RopeSpline`)))))
    (set `self.CurrentDistanceOnRope` (`KismetMathLibrary.FClamp` (+ (`self.CurrentDistanceOnRope`) (* (`local.DeltaSec`) (`self.WalkSpeedPerSeconds`) (`self.CurrentSpeedMultiplier`))) 0.0 (`self.GoalDistanceOnRope`)))
    (`KismetSystemLibrary.PrintString` (`KismetStringLibrary.Concat_StrStr` "Affected Speed Multiplier" (`KismetStringLibrary.Conv_DoubleToString` (`self.CurrentSpeedMultiplier`))) true true (struct :`R` 0.935843 :`G` 1.0 :`A` 1.0) 0.0)
    (else
      (set `self.IsBenMoving` false))))

(fn `UserConstructionScript`)