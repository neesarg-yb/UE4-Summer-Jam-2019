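; Ben is a player-controlled tightrope walker who moves along the level's RopeSpline and must keep his balance.
; Each Tick, W/S drive linear velocity with friction and A/D drive tilt velocity, using tuning values loaded from the Ben2MovementForces data table.
; A self-rescheduling timer triggers random left or right wind-like gusts that add rotational force.
; Tilting past the fall threshold marks Ben fallen, hides his mesh and halts movement.
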(event `self.ReceiveBeginPlay`
  (`|ExecutionSequence`
    (:`then_0`
      (`self.SetVariablesFromDataTables`)
      (bind _outactors (`GameplayStatics.GetAllActorsOfClass` "/Game/Blueprints/RopeSpline.RopeSpline_C"))
      (bind _output_get (set `self.RopeSpline` (`|GetArrayItem` _outactors)))
      (`self.K2_SetActorTransform` (`SplineComponent.GetTransformAtDistanceAlongSpline` (`/Game/Blueprints/RopeSpline.Spline` _output_get) 0.0 "World" false) false true))
    (:`then_1`
      (`KismetSystemLibrary.K2_SetTimerDelegate` (delegate `LoseControlForceTimerDue`) (`self.MinNextLoseControlAfterSeconds_Const`)))
    (:`then_2`
      (`self.InitalizeGroceriesInHands`))))

(event `LoseControlForceTimerDue`
  (`|ExecutionSequence`
    (:`then_0`
      (if (<= (`KismetMathLibrary.RandomIntegerInRange` 0 100) 50)
        (set `self.LoseControlForceDirectionMult` 1.0)
        (else
          (set `self.LoseControlForceDirectionMult` -1.0))))
    (:`then_1`
      (bind _output_get (set `self.LastWindForceTotalDuration` (`KismetMathLibrary.RandomFloatInRange` (`self.MinLoseControlForceDuration_Const`) (`self.MaxLoseControlForceDuration_Const`))))
      (bind _output_get_2 (set `self.RemainingDuration_LoseControlForce` _output_get))
      (`KismetSystemLibrary.K2_SetTimerDelegate` (delegate `LoseControlForceTimerDue`) (+ _output_get_2 (`KismetMathLibrary.RandomFloatInRange` (`self.MinNextLoseControlAfterSeconds_Const`) (`self.MaxNextLoseControlAfterSeconds_Const`)))))))

(event `self.ReceiveTick`
  (params (DeltaSeconds :type "Float (single-precision)"))
  (if (`self.BenAlreadyFellDown`)
    (`SceneComponent.SetVisibility` (`self.Ben_SkeletonMesh`) false true)
    (else
      (`self.ClearLastFramesForces`)
      (`self.UpdateInput`)
      (`self.UpdateLinearVelocity` DeltaSeconds)
      (`self.ApplyRandomLoseControlForce` DeltaSeconds)
      (`self.UpdateRotationalVelocity` DeltaSeconds)
      (`self.MoveBenOnRope` DeltaSeconds)
      (`self.RotateBenAlongTheRope` DeltaSeconds)
      (`self.UpdateBenStaticMeshRotation`)
      (`self.CheckIfBenFell`))))

(event `BenJustFellDown`
  (`KismetSystemLibrary.PrintString` "BEN JUST FELL DOWN!" true true (struct :`R` 1.0 :`B` 0.026892 :`A` 1.0) 15.0))

(fn `AddRotationalForce`
  (params (RotationalForce :type "Float (double-precision)"))
  (set `self.RotationalForceThisFrame` (+ RotationalForce (`self.RotationalForceThisFrame`))))

(fn `ApplyRandomLoseControlForce`
  (params (DeltaSeconds :type "Float (double-precision)"))
  (locals (DeltaSec :type "Float (double-precision)"))
  (set `local.DeltaSec` DeltaSeconds)
  (if (> (`self.RemainingDuration_LoseControlForce`) 0.0)
    (`self.AddRotationalForce` (* (`self.RandomLoseControlForce_Const`) (`self.LoseControlForceDirectionMult`)))
    (set `self.RemainingDuration_LoseControlForce` (- (`self.RemainingDuration_LoseControlForce`) (`local.DeltaSec`)))))

(fn `CheckIfBenFell`
  (locals (PreviousBenFellValue :type Boolean))
  (set `local.PreviousBenFellValue` (`self.BenAlreadyFellDown`))
  (bind _output_get (set `self.BenAlreadyFellDown` (>= (`KismetMathLibrary.Abs` (`self.CurrentVerticalOffsetDegrees`)) (`self.FallThresholdDegrees_Const`))))
  (if _output_get
    (if (not (`local.PreviousBenFellValue`))
      (`self.BenJustFellDown`))))

(fn `ClearLastFramesForces`
  (set `self.LinearWillpowerForceThisFrame` 0.0)
  (set `self.RotationalForceThisFrame` 0.0))

(fn `DebugRenderBen`
  (bind _fallthresholddegrees_const (`self.FallThresholdDegrees_Const`))
  (bind _returnvalue (`SceneComponent.K2_GetComponentLocation` (`self.DefaultSceneRoot`)))
  (bind _returnvalue_2 (`SceneComponent.GetForwardVector` (`self.DefaultSceneRoot`)))
  (bind _returnvalue_3 (`SceneComponent.K2_GetComponentLocation` (`self.DefaultSceneRoot`)))
  (bind _returnvalue_4 (`KismetMathLibrary.MakeVector` 0.0 0.0 (* (`self.BodyLength`) 1.25)))
  (`|ExecutionSequence`
    (:`then_0`
      (`KismetSystemLibrary.DrawDebugLine` _returnvalue_3 (+ _returnvalue_3 (`KismetMathLibrary.RotateAngleAxis` (`KismetMathLibrary.MakeVector` 0.0 0.0 (`self.BodyLength`)) (`self.CurrentVerticalOffsetDegrees`) (`SceneComponent.GetForwardVector` (`self.DefaultSceneRoot`)))) (struct :`R` 0.469453 :`B` 1.0 :`A` 1.0) 0.0 25.0))
    (:`then_1`
      (`|ExecutionSequence`
        (:`then_0`
          (`KismetSystemLibrary.DrawDebugLine` _returnvalue (+ _returnvalue (`KismetMathLibrary.RotateAngleAxis` _returnvalue_4 _fallthresholddegrees_const _returnvalue_2)) (struct :`R` 1.0 :`B` 0.016003 :`A` 1.0) 0.0 1.0))
        (:`then_1`
          (`KismetSystemLibrary.DrawDebugLine` _returnvalue (+ _returnvalue (`KismetMathLibrary.RotateAngleAxis` _returnvalue_4 (* _fallthresholddegrees_const -1.0) _returnvalue_2)) (struct :`R` 1.0 :`B` 0.016003 :`A` 1.0) 0.0 1.0))))))

(fn `InitalizeGroceriesInHands`)

(fn `IsWindActive`
  (returns (IsActive :type Boolean) (Direction :type "Float (double-precision)") (ActivatedForTotalDuration :type "Float (double-precision)"))
  (return (> (`self.RemainingDuration_LoseControlForce`) 0.0) (`self.LoseControlForceDirectionMult`) (`self.LastWindForceTotalDuration`)))

(fn `MoveBenOnRope`
  (params (DeltaSeconds :type "Float (double-precision)"))
  (set `self.LinearPosition` (+ (* DeltaSeconds (`self.LinearVelocity`)) (`self.LinearPosition`)))
  (`self.K2_SetActorTransform` (`SplineComponent.GetTransformAtDistanceAlongSpline` (`/Game/Blueprints/RopeSpline.Spline` (`self.RopeSpline`)) (`self.LinearPosition`) "World" false)))

(fn `RotateBenAlongTheRope`
  (params (DeltaSeconds :type "Float (double-precision)"))
  (set `self.CurrentVerticalOffsetDegrees` (+ (`self.CurrentVerticalOffsetDegrees`) (* DeltaSeconds (`self.RotationalVelocity`)))))

(fn `SetVariablesFromDataTables`
  (`|ExecutionSequence`
    (:`then_0`
      (bind _returnvalue (`|GetDataTableRow` "/Game/DataTables/Ben-2/Ben-2-MovementForces.Ben-2-MovementForces" "LinearMovementForce")
        (:`then`
          (set `self.WillPowerForce_Const` (break `/Game/DataStructures/FloatStructure` _returnvalue)))
        (:`RowNotFound`
          (`KismetSystemLibrary.PrintString` "Warning: DATA TABLE ROW LinearMovementForce NOT FOUND" true true (struct :`R` 1.0 :`B` 0.064835 :`A` 1.0) 5.0))))
    (:`then_1`
      (bind _returnvalue_2 (`|GetDataTableRow` "/Game/DataTables/Ben-2/Ben-2-MovementForces.Ben-2-MovementForces" "FrictionScale")
        (:`then`
          (set `self.FrictionScale_Const` (break `/Game/DataStructures/FloatStructure` _returnvalue_2)))
        (:`RowNotFound`
          (`KismetSystemLibrary.PrintString` "Warning: DATA TABLE ROW FrictionScale NOT FOUND" true true (struct :`R` 1.0 :`B` 0.064835 :`A` 1.0) 5.0))))
    (:`then_2`
      (bind _returnvalue_3 (`|GetDataTableRow` "/Game/DataTables/Ben-2/Ben-2-MovementForces.Ben-2-MovementForces" "LinearMaxSpeed")
        (:`then`
          (set `self.LinearMaxSpeed_Const` (break `/Game/DataStructures/FloatStructure` _returnvalue_3)))
        (:`RowNotFound`
          (`KismetSystemLibrary.PrintString` "Warning: DATA TABLE ROW LinearMaxSpeed NOT FOUND" true true (struct :`R` 1.0 :`B` 0.064835 :`A` 1.0) 5.0))))
    (:`then_3`
      (bind _returnvalue_4 (`|GetDataTableRow` "/Game/DataTables/Ben-2/Ben-2-MovementForces.Ben-2-MovementForces" "RotationWillpowerForce")
        (:`then`
          (set `self.RotationWillPowerForce_Const` (break `/Game/DataStructures/FloatStructure` _returnvalue_4)))
        (:`RowNotFound`
          (`KismetSystemLibrary.PrintString` "Warning: DATA TABLE ROW RotationWillpowerForce NOT FOUND" true true (struct :`R` 1.0 :`B` 0.064835 :`A` 1.0) 5.0))))
    (:`then_4`
      (bind _returnvalue_5 (`|GetDataTableRow` "/Game/DataTables/Ben-2/Ben-2-MovementForces.Ben-2-MovementForces" "FallThresholdDegrees")
        (:`then`
          (set `self.FallThresholdDegrees_Const` (break `/Game/DataStructures/FloatStructure` _returnvalue_5)))
        (:`RowNotFound`
          (`KismetSystemLibrary.PrintString` "Warning: DATA TABLE ROW FallThresholdDegrees NOT FOUND" true true (struct :`R` 1.0 :`B` 0.064835 :`A` 1.0) 5.0))))
    (:`then_5`
      (bind _returnvalue_6 (`|GetDataTableRow` "/Game/DataTables/Ben-2/Ben-2-MovementForces.Ben-2-MovementForces" "RandomlyLoseControlForce")
        (:`then`
          (set `self.RandomLoseControlForce_Const` (break `/Game/DataStructures/FloatStructure` _returnvalue_6)))
        (:`RowNotFound`
          (`KismetSystemLibrary.PrintString` "Warning: DATA TABLE ROW RandomlyLoseControlForce NOT FOUND" true true (struct :`R` 1.0 :`B` 0.064835 :`A` 1.0) 5.0))))
    (:`then_6`
      (bind _returnvalue_7 (`|GetDataTableRow` "/Game/DataTables/Ben-2/Ben-2-MovementForces.Ben-2-MovementForces" "MinLoseControlDuration")
        (:`then`
          (set `self.MinLoseControlForceDuration_Const` (break `/Game/DataStructures/FloatStructure` _returnvalue_7)))
        (:`RowNotFound`
          (`KismetSystemLibrary.PrintString` "Warning: DATA TABLE ROW MinLoseControlForceDuration NOT FOUND" true true (struct :`R` 1.0 :`B` 0.064835 :`A` 1.0) 5.0))))
    (:`then_7`
      (bind _returnvalue_8 (`|GetDataTableRow` "/Game/DataTables/Ben-2/Ben-2-MovementForces.Ben-2-MovementForces" "MaxLoseControlDuration")
        (:`then`
          (set `self.MaxLoseControlForceDuration_Const` (break `/Game/DataStructures/FloatStructure` _returnvalue_8)))
        (:`RowNotFound`
          (`KismetSystemLibrary.PrintString` "Warning: DATA TABLE ROW MaxLoseControlDuration NOT FOUND" true true (struct :`R` 1.0 :`B` 0.064835 :`A` 1.0) 5.0))))
    (:`then_8`
      (bind _returnvalue_9 (`|GetDataTableRow` "/Game/DataTables/Ben-2/Ben-2-MovementForces.Ben-2-MovementForces" "MinNextLoseControlAfterDuration")
        (:`then`
          (set `self.MinNextLoseControlAfterSeconds_Const` (break `/Game/DataStructures/FloatStructure` _returnvalue_9)))
        (:`RowNotFound`
          (`KismetSystemLibrary.PrintString` "Warning: DATA TABLE ROW MinNextLoseControlAfterSeconds NOT FOUND" true true (struct :`R` 1.0 :`B` 0.064835 :`A` 1.0) 5.0))))
    (:`then_9`
      (bind _returnvalue_10 (`|GetDataTableRow` "/Game/DataTables/Ben-2/Ben-2-MovementForces.Ben-2-MovementForces" "MaxNextLoseControlAfterDuration")
        (:`then`
          (set `self.MaxNextLoseControlAfterSeconds_Const` (break `/Game/DataStructures/FloatStructure` _returnvalue_10)))
        (:`RowNotFound`
          (`KismetSystemLibrary.PrintString` "Warning: DATA TABLE ROW MaxLoseControlAfterSeconds NOT FOUND" true true (struct :`R` 1.0 :`B` 0.064835 :`A` 1.0) 5.0))))))

(fn `UpdateBenPositionFallingDown`)

(fn `UpdateBenStaticMeshRotation`
  (bind (_returnvalue_roll _returnvalue_pitch _returnvalue_yaw) (`KismetMathLibrary.BreakRotator` (`SceneComponent.K2_GetComponentRotation` (`self.Ben_SkeletonMesh`))))
  (`SceneComponent.K2_SetWorldRotation` (`self.Ben_SkeletonMesh`) (`KismetMathLibrary.MakeRotator` _returnvalue_roll (* (`self.CurrentVerticalOffsetDegrees`) -1.0) _returnvalue_yaw) false false))

(fn `UpdateInput`
  (`|ExecutionSequence`
    (:`then_0`
      (if (`PlayerController.IsInputKeyDown` (`GameplayStatics.GetPlayerController` 0) "W")
        (set `self.LinearWillpowerForceThisFrame` (+ (`self.LinearWillpowerForceThisFrame`) (`self.WillPowerForce_Const`)))))
    (:`then_1`
      (if (`PlayerController.IsInputKeyDown` (`GameplayStatics.GetPlayerController` 0) "S")
        (set `self.LinearWillpowerForceThisFrame` (* -1.0 (+ (`self.LinearWillpowerForceThisFrame`) (`self.WillPowerForce_Const`))))))
    (:`then_2`
      (if (`PlayerController.IsInputKeyDown` (`GameplayStatics.GetPlayerController` 0) "A")
        (set `self.RotationalForceThisFrame` (`self.RotationWillPowerForce_Const`))))
    (:`then_3`
      (if (`PlayerController.IsInputKeyDown` (`GameplayStatics.GetPlayerController` 0) "D")
        (set `self.RotationalForceThisFrame` (* (`self.RotationWillPowerForce_Const`) -1.0))))))

(fn `UpdateLinearVelocity`
  (params (DeltaSeconds :type "Float (double-precision)"))
  (locals (LinearFriction :type "Float (double-precision)") (LinearTotalForce :type "Float (double-precision)") (DeltaVelocity :type "Float (double-precision)") (DeltaSec :type "Float (double-precision)"))
  (set `local.DeltaSec` DeltaSeconds)
  (`|ExecutionSequence`
    (:`then_0`
      (bind _output_get (set `local.LinearFriction` (* (`self.LinearVelocity`) (`self.FrictionScale_Const`) -1.0))))
    (:`then_1`
      (bind _output_get_2 (set `local.LinearTotalForce` (+ (`self.LinearWillpowerForceThisFrame`) (`local.LinearFriction`)))))
    (:`then_2`
      (set `local.DeltaVelocity` (* (`local.LinearTotalForce`) (`local.DeltaSec`))))
    (:`then_3`
      (bind _output_get_3 (set `self.LinearVelocity` (+ (`self.LinearVelocity`) (`local.DeltaVelocity`)))))
    (:`then_4`
      (set `self.LinearVelocity` (* (`KismetMathLibrary.SignOfFloat` (`self.LinearVelocity`)) (`KismetMathLibrary.FClamp` (`KismetMathLibrary.Abs` (`self.LinearVelocity`)) 0.0 (`self.LinearMaxSpeed_Const`)))))))

(fn `UpdateRotationalVelocity`
  (params (DeltaSeconds :type "Float (double-precision)"))
  (locals (RotationalDeltaVelocity :type "Float (double-precision)") (DeltaSec :type "Float (double-precision)"))
  (set `local.DeltaSec` DeltaSeconds)
  (`|ExecutionSequence`
    (:`then_0`
      (set `local.RotationalDeltaVelocity` (* (`self.RotationalForceThisFrame`) (`local.DeltaSec`))))
    (:`then_1`
      (set `self.RotationalVelocity` (+ (`self.RotationalVelocity`) (`local.RotationalDeltaVelocity`))))))

(fn `UserConstructionScript`)