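; BenOnSpline is an actor that travels along the spline of a referenced rope actor, automatically at BeginPlay when enabled.
; MoveBen plays a timeline rate-scaled by a duration, mapping its alpha to distance along the spline.
; The spline's local-space location and rotation are applied directly as the actor's world transform.
; Each tick draws a debug body line from the root, tilted about world X.
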(event `self.ReceiveBeginPlay`
  (if (`self.EnabledAutoMovement`)
    (`self.MoveBen`)))

(event `self.ReceiveTick`
  (params (DeltaSeconds :type "Float (single-precision)"))
  (`self.DebugRenderBodyLine`))

(event `MoveBen`
  (bind (_returnvalue_location _returnvalue_rotation) (`KismetMathLibrary.BreakTransform` (`SplineComponent.GetTransformAtDistanceAlongSpline` (`/Game/Blueprints/RopeSpline.Spline` (`self.RopeSpineRef`)) (`KismetMathLibrary.Lerp` 0.0 (`SplineComponent.GetSplineLength` (`/Game/Blueprints/RopeSpline.Spline` (`self.RopeSpineRef`))) (`self.MovementAlphaFraction`)) "Local" false)))
  (`TimelineComponent.SetPlayRate` (`self.BenAutoMovementTimeline`) (/ 1.0 (`self.Duration Seconds`)))
  (bind (_direction _alpha) (`Timeline|BenAutoMovementTimeline`)
    (:`Update`
      (set `self.MovementAlphaFraction` _alpha)
      (`self.K2_SetActorTransform` (`KismetMathLibrary.MakeTransform` _returnvalue_location _returnvalue_rotation)))))

(fn `DebugRenderBodyLine`
  (locals (BodyLength :type "Float (double-precision)" :default 180.0))
  (bind _returnvalue (`SceneComponent.K2_GetComponentLocation` (`self.DefaultSceneRoot`)))
  (`KismetSystemLibrary.DrawDebugLine` _returnvalue (+ _returnvalue (`KismetMathLibrary.RotateAngleAxis` (`KismetMathLibrary.MakeVector` 0.0 0.0 (`local.BodyLength`)) (`self.OffsetVerticalDegrees`) (1.0 0.0 0.0))) (struct :`R` 0.500624 :`G` 0.500969 :`B` 1.0 :`A` 1.0) 0.0 25.0))

(fn `UserConstructionScript`)