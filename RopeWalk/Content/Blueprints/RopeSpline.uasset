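; RopeSpline is an actor that builds a rope-like mesh along an editable spline, with no active runtime logic.
; Its construction script adds a spline mesh component for each segment between consecutive spline points, using a configurable static mesh and forward axis.
; Each piece is attached to the spline, bent with local point locations and tangents, and given query and physics collision.
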(fn `UserConstructionScript`
  (for _index (range (+ (- (`SplineComponent.GetNumberOfSplinePoints` (`self.Spline`)) 2) 1))
    (bind _returnvalue (`AddComponent|NODE_AddSplineMeshComponent-0`))
    (`|ExecutionSequence`
      (:`then_0`
        (`StaticMeshComponent.SetStaticMesh` _returnvalue (`self.StaticMesh`))
        (`SplineMeshComponent.SetForwardAxis` _returnvalue (`self.ForwardAxis`) true)
        (`PrimitiveComponent.SetCollisionEnabled` _returnvalue "QueryAndPhysics"))
      (:`then_1`
        (`SceneComponent.K2_AttachToComponent` _returnvalue (`self.Spline`) "None" "KeepRelative" "KeepRelative" "KeepRelative" true)
        (bind _returnvalue_2 (+ _index 1))
        (`SplineMeshComponent.SetStartAndEnd` _returnvalue (`SplineComponent.GetLocationAtSplinePoint` (`self.Spline`) _index "Local") (`SplineComponent.GetTangentAtSplinePoint` (`self.Spline`) _index "Local") (`SplineComponent.GetLocationAtSplinePoint` (`self.Spline`) _returnvalue_2 "Local") (`SplineComponent.GetTangentAtSplinePoint` (`self.Spline`) _returnvalue_2 "Local") true)))))